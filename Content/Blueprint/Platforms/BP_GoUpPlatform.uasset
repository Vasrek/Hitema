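; Platform actor that rises to a target location and returns to its starting position.
; BeginPlay saves the start location as DefaultLocation.
; StartMoveUp and StartMoveDown each wait briefly, then start a fast looping timer by function name.
; MoveUp and MoveDown ease the actor toward LocationToReach or DefaultLocation with VInterpTo, without sweep, and clear their timer within a loose tolerance instead of snapping to the target.
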(event `self.ReceiveBeginPlay`
  ;[1 1 1] Save default location
  (set `self.DefaultLocation` (`self.K2_GetActorLocation`)))

(event `StartMoveDown`
  ;[1 1 1] After 3 seconds, go down
  (`KismetSystemLibrary.Delay` 3.0)
  (`KismetSystemLibrary.K2_SetTimer` null "MoveDown" 0.01 true))

(event `StartMoveUp`
  ;[1 1 1] After 3 seconds, go up
  (`KismetSystemLibrary.Delay` 3.0)
  (`KismetSystemLibrary.K2_SetTimer` null "MoveUp" 0.01 true))

(fn `MoveDown`
  (bind _returnvalue (`KismetMathLibrary.VInterpTo` (`self.K2_GetActorLocation`) (`self.DefaultLocation`) (`GameplayStatics.GetWorldDeltaSeconds`) (`self.InterpSpeed`)))
  (`self.K2_SetActorLocation` _returnvalue)
  (if (== _returnvalue (`self.DefaultLocation`) :`ErrorTolerance` 50.0)
    (`KismetSystemLibrary.K2_ClearTimer` null "MoveDown")))

(fn `MoveUp`
  (bind _returnvalue (`KismetMathLibrary.VInterpTo` (`self.K2_GetActorLocation`) (`self.LocationToReach`) (`GameplayStatics.GetWorldDeltaSeconds`) (`self.InterpSpeed`)))
  (`self.K2_SetActorLocation` _returnvalue)
  (if (== _returnvalue (`self.LocationToReach`) :`ErrorTolerance` 50.0)
    (`KismetSystemLibrary.K2_ClearTimer` null "MoveUp")))

(fn `UserConstructionScript`)