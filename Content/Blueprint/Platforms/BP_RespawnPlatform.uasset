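; Checkpoint platform that sets the player's respawn point and then rides up or down.
; On begin play it caches the arrow component's world transform as the new respawn transform.
; When a BP_Player overlaps the box, it stores that transform on the player, adds score, and plays a checkpoint sound with a brief spark burst.
; The GoesUp flag chooses whether the linked Platform starts moving up or down.
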(event `self.ReceiveBeginPlay`
  ;[1 1 1] Save arrow transform (new transform for respawn player)
  (set `self.NewRespawnTransform` (`SceneComponent.K2_GetComponentToWorld` (`self.Arrow`))))

(event `self.Box.OnComponentBeginOverlap`
  (params (OverlappedComponent :type "PrimitiveComponent Object Reference") (OtherActor :type "Actor Object Reference") (OtherComp :type "PrimitiveComponent Object Reference") (OtherBodyIndex :type Integer) (bFromSweep :type Boolean) (SweepResult :type "HitResult Structure (by ref)"))
  ;[1 1 1] If player goes into trigger -> set new respawn transform and call elevator
  (bind _asbp_player (cast `/Game/Blueprint/Character/BP_Player` OtherActor))
  (`ActorComponent.Activate` (`self.P_Sparks`) false)
  (`GameplayStatics.PlaySound2D` "/Game/Audio/Checkpoint_Sound_Effect.Checkpoint_Sound_Effect" 1.0 1.0 0.0 null null)
  (set `/Game/Blueprint/Character/BP_Player.RespawnLocation` (`self.NewRespawnTransform`) _asbp_player)
  (`/Game/Blueprint/Character/BP_Player.IncreaseScore` _asbp_player 10)
  (if (`self.GoesUp?`)
    (`/Game/Blueprint/Platforms/BP_GoUpPlatform.StartMoveUp` (`self.Platform`))
    (else
      (`/Game/Blueprint/Platforms/BP_GoUpPlatform.StartMoveDown` (`self.Platform`))))
  (`KismetSystemLibrary.Delay` 1.5)
  (`ActorComponent.Deactivate` (`self.P_Sparks`)))

(fn `UserConstructionScript`)